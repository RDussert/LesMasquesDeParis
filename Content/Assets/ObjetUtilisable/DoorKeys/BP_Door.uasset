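; BP_Door is a hinged door that swings open and closed each time its Interract event is triggered.
; A Box overlap sets InRangeDoor on BP_FirstPersonCharacter while it is inside and clears it on exit.
; Interract uses a FlipFlop to alternate between playing the DoorOpen timeline from start and reversing it, lerping the Door's relative yaw through a quarter turn.
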(event OnComponentBeginOverlap(Box)
  (params (OverlappedComponent :type Primitive%20Component%20Object%20Reference) (OtherActor :type Actor%20Object%20Reference) (OtherComp :type Primitive%20Component%20Object%20Reference) (OtherBodyIndex :type Integer) (bFromSweep :type Boolean) (SweepResult :type Hit%20Result%20Structure%20%28by%20ref%29))
  (bind _asbp_first_person_character (Utilities|Casting|CastToBP_FirstPersonCharacter OtherActor))
  (Variables|/Game/FirstPerson/Blueprints/BP_FirstPersonCharacter.BP_FirstPersonCharacter_C|SetInRangeDoor _asbp_first_person_character true))

(event OnComponentEndOverlap(Box)
  (params (OverlappedComponent :type Primitive%20Component%20Object%20Reference) (OtherActor :type Actor%20Object%20Reference) (OtherComp :type Primitive%20Component%20Object%20Reference) (OtherBodyIndex :type Integer))
  (bind _asbp_first_person_character (Utilities|Casting|CastToBP_FirstPersonCharacter OtherActor))
  (Variables|/Game/FirstPerson/Blueprints/BP_FirstPersonCharacter.BP_FirstPersonCharacter_C|SetInRangeDoor _asbp_first_person_character false))

(event EventBeginPlay)

(event Collision|EventActorBeginOverlap
  (params (OtherActor :type Actor%20Object%20Reference)))

(event EventTick
  (params (DeltaSeconds :type Float%20%28single-precision%29)))

(event EventInterract
  (Utilities|FlowControl|FlipFlop
    (:A
      (bind _doorfloat (Timeline|DoorOpen PlayFromStart)
        (:Update
          (Transformation|SetRelativeRotation (Variables|Default|GetDoor) (Math|Rotator|MakeRotator 0.0 0.0 (Math|Float|Lerp 0.0 -9e+01 _doorfloat)) false false))))
    (:B
      (Timeline|DoorOpen Reverse))))

(fn ConstructionScript)