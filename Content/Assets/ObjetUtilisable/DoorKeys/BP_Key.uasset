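; BP_Key is an interactable key pickup that the player can highlight and collect.
; Highlight toggles an overlay material on the key mesh.
; Interract plays pickup audio, shows a WB_KeyPickUp widget with the key's description, adds the key to the pocket and destroys the actor.
; AddToPocket appends the key's name and photo to the KeysInPocket and KeysPictures arrays on BP_FirstPersonCharacter.
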(event EventBeginPlay)

(event Collision|EventActorBeginOverlap
  (params (OtherActor :type Actor%20Object%20Reference)))

(event EventTick
  (params (DeltaSeconds :type Float%20%28single-precision%29)))

(event EventInterract
  (Audio|PlaySound2D "/Game/Assets/EventScripts/Event_Sounds_Ambience/SC_KeyPick.SC_KeyPick" 1.0 1.0 0.0 0 0)
  (bind _returnvalue (UserInterface|CreateWidget "/Game/UserInterface/WB_KeyPickUp.WB_KeyPickUp_C" 0 (Variables|Default|GetDescritpionOfKey)))
  (UserInterface|Viewport|AddtoViewport _returnvalue 0)
  (Audio|PlaySound2D 0 1.0 1.0 0.0 0 0)
  (CallFunction|AddtoPocket)
  (Actor|DestroyActor))

(event EventHighlight
  (params (Highlight? :type Boolean))
  (if Highlight?
    (Rendering|Material|SetOverlayMaterial (Variables|Default|GetSM_Key) "/Game/Material/M_Highlight_Objects.M_Highlight_Objects" :!class /Script/Engine.MeshComponent)
    (else
      (Rendering|Material|SetOverlayMaterial (Variables|Default|GetSM_Key) 0 :!class /Script/Engine.MeshComponent))))

(fn ConstructionScript)

(fn AddtoPocket
  (bind _asbp_first_person_character (Utilities|Casting|CastToBP_FirstPersonCharacter (Game|GetPlayerCharacter 0)))
  (Utilities|Array|Add (Variables|/Game/FirstPerson/Blueprints/BP_FirstPersonCharacter.BP_FirstPersonCharacter_C|GetKeysInPocket _asbp_first_person_character) (Variables|Default|GetNameOfKey))
  (Utilities|Array|Add (Variables|/Game/FirstPerson/Blueprints/BP_FirstPersonCharacter.BP_FirstPersonCharacter_C|GetKeysPictures _asbp_first_person_character) (Variables|Default|GetPhoto)))