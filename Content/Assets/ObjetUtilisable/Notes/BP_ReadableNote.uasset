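; BP_ReadableNote is a note actor the player can read by interacting with it.
; Interract toggles between pick-up and put-down, each playing its own sound.
; Picking up shows a WB_Notes widget with the note's text, hides the actor and turns off player input through SetInput on BP_FirstPersonCharacter; putting down reverses this.
; Leftover proximity logic around IsCloseEnough is disconnected and never runs.
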(event Custom|TogglePickUp
  (if (Variables|Default|GetIsReading?)
    (CallFunction|PutDownNote)
    (else
      (CallFunction|PickUpNote))))

(event Custom|PickUpNote
  (Audio|SpawnSound2D "/Game/Assets/ObjetUtilisable/Notes/NoteSounds/Note_PickUp.Note_PickUp" 1.0 1.0 0.0 0)
  (bind _returnvalue (UserInterface|CreateWidget "/Game/Assets/ObjetUtilisable/Notes/WB_Notes.WB_Notes_C" 0 (Variables|Default|GetText%20Of%20Note)))
  (UserInterface|Viewport|AddtoViewport _returnvalue 0)
  (Variables|Default|SetIsReading? true)
  (Rendering|SetActorHiddenInGame true)
  (Default|SetInput (Variables|Default|GetAs%20BP%20First%20Person%20Character) false))

(event Custom|PutDownNote
  (Audio|SpawnSound2D "/Game/Assets/ObjetUtilisable/Notes/NoteSounds/Note_PutDown2.Note_PutDown2" 1.0 1.0 0.0 0)
  (Widget|RemovefromParent (stale Custom|PickUpNote _returnvalue))
  (Variables|Default|SetIsReading? false)
  (Rendering|SetActorHiddenInGame false)
  (Default|SetInput (Variables|Default|GetAs%20BP%20First%20Person%20Character) true))

(event EventInterract
  (CallFunction|TogglePickUp))

(event EventBeginPlay
  (bind _asbp_first_person_character (Utilities|Casting|CastToBP_FirstPersonCharacter (Game|GetPlayerCharacter 0)))
  (Variables|Default|SetAs%20BP%20First%20Person%20Character _asbp_first_person_character))

(fn ConstructionScript)