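; BP_Door is a door Blueprint that moves automatically when its Box trigger is overlapped.
; Begin and end overlap share one FlipFlop, so each overlap event alternates between open and close without checking which actor triggered it.
; The open/close event briefly activates one of two RotatingMovement components, then deactivates it after a fixed Delay, so rotation is timed rather than driven to a target angle.
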(event OnComponentBeginOverlap(Box)
  (params (OverlappedComponent :type Primitive%20Component%20Object%20Reference) (OtherActor :type Actor%20Object%20Reference) (OtherComp :type Primitive%20Component%20Object%20Reference) (OtherBodyIndex :type Integer) (bFromSweep :type Boolean) (SweepResult :type Hit%20Result%20Structure%20%28by%20ref%29))
  (Utilities|FlowControl|FlipFlop
    (:A
      (CallFunction|Open/Closee true))
    (:B
      (CallFunction|Open/Closee false))))

(event OnComponentEndOverlap(Box)
  (params (OverlappedComponent :type Primitive%20Component%20Object%20Reference) (OtherActor :type Actor%20Object%20Reference) (OtherComp :type Primitive%20Component%20Object%20Reference) (OtherBodyIndex :type Integer))
  (Utilities|FlowControl|FlipFlop
    (:A
      (CallFunction|Open/Closee true))
    (:B
      (CallFunction|Open/Closee false))))

(event Custom|Open/Closee
  (params (Open? :type Boolean))
  (bind _rotatingmovement (Variables|Default|GetRotatingMovement))
  (bind _rotatingmovement1 (Variables|Default|GetRotatingMovement1))
  (if Open?
    (Components|Activation|Activate _rotatingmovement false)
    (Utilities|FlowControl|Delay 1.0)
    (Components|Activation|Deactivate _rotatingmovement)
    (else
      (Components|Activation|Activate _rotatingmovement1 false)
      (Utilities|FlowControl|Delay 1.0)
      (Components|Activation|Deactivate _rotatingmovement1))))

(event EventBeginPlay)

(event Collision|EventActorBeginOverlap
  (params (OtherActor :type Actor%20Object%20Reference)))

(event EventTick
  (params (DeltaSeconds :type Float%20%28single-precision%29)))

(fn ConstructionScript)