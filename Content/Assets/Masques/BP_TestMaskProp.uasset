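; BP_TestMaskProp is a test prop that vanishes and loses collision while the player wears a mask.
; One tick after BeginPlay, it casts the player pawn to BP_FirstPersonCharacter and binds Set_Real to that character's PrintText dispatcher.
; Each dispatch runs MaskVerification, which reads WearMask and toggles the static mesh's visibility and collision to match.
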(event Custom|Set_Real
  (CallFunction|MaskVerification (Variables|Default|GetCharacter)))

(event EventBeginPlay
  (Utilities|FlowControl|DelayUntilNextTick)
  (bind _asbp_first_person_character (Utilities|Casting|CastToBP_FirstPersonCharacter (Game|GetPlayerCharacter 0)))
  (bind _output_get (Variables|Default|SetCharacter _asbp_first_person_character))
  (EventDispatchers|BindEventtoPrintText _output_get (delegate Custom|Set_Real)))

(event Collision|EventActorBeginOverlap
  (params (OtherActor :type Actor%20Object%20Reference)))

(event EventTick
  (params (DeltaSeconds :type Float%20%28single-precision%29)))

(fn ConstructionScript)

(fn MaskVerification
  (params (Character%20 :type BP%20First%20Person%20Character%20Object%20Reference))
  (bind _staticmesh (Variables|Default|GetStaticMesh))
  (bind _staticmesh_2 (Variables|Default|GetStaticMesh))
  (if (Variables|/Game/FirstPerson/Blueprints/BP_FirstPersonCharacter.BP_FirstPersonCharacter_C|GetWearMask Character%20)
    (Collision|SetCollisionEnabled _staticmesh "NoCollision")
    (Development|SetHiddeninGame _staticmesh true false)
    (else
      (Collision|SetCollisionEnabled _staticmesh_2 "QueryAndPhysics")
      (Development|SetHiddeninGame _staticmesh_2 false false))))