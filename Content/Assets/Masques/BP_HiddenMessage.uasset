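; Hidden clue actor that shows its text only while the player wears the mask.
; On BeginPlay it writes Message to its TextRender, caches the first-person character and binds to that character's PrintText dispatcher.
; Each dispatcher call runs MaskVerification, which shows or hides the text in game based on the character's WearMask flag.
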(event Custom|set_visible
  ;[1 1 1] On Vérifie si le joueur porte le masque
  (CallFunction|MaskVerification (Variables|Default|GetCharacter)))

(event Collision|EventActorBeginOverlap
  (params (OtherActor :type Actor%20Object%20Reference)))

(event EventTick
  (params (DeltaSeconds :type Float%20%28single-precision%29)))

(event EventBeginPlay
  ;[1 1 1] On set le texte des indices cachés
  (Rendering|Components|TextRender|SetText (Variables|Default|GetTextRender) (Variables|Default|GetMessage))
  ;[1 1 1] On Vérifie si le joueur porte le masque
  (bind _asbp_first_person_character (Utilities|Casting|CastToBP_FirstPersonCharacter (Game|GetPlayerCharacter 0)))
  (bind _output_get (Variables|Default|SetCharacter _asbp_first_person_character))
  (EventDispatchers|BindEventtoPrintText _output_get (delegate Custom|set_visible)))

(fn ConstructionScript)

(fn MaskVerification
  (params (Character :type BP%20First%20Person%20Character%20Object%20Reference))
  (if (Variables|/Game/FirstPerson/Blueprints/BP_FirstPersonCharacter.BP_FirstPersonCharacter_C|GetWearMask Character)
    (Development|SetHiddeninGame (Variables|Default|GetTextRender) false false)
    (else
      (Development|SetHiddeninGame (Variables|Default|GetTextRender) true false))))