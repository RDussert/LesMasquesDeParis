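; BP_Mask is a mask pickup actor that the player collects by interacting with it.
; On interact, it plays the key pickup sound, sets HasMask on the first-person character, then destroys itself.
; A Highlight event toggles an overlay material on its plane mesh to mark it as highlighted.
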(event EventHighlight
  (params (Highlight? :type Boolean))
  (if Highlight?
    (Rendering|Material|SetOverlayMaterial (Variables|Default|GetPlane) "/Game/Material/M_Highlight_Objects.M_Highlight_Objects" :!class /Script/Engine.MeshComponent)
    (else
      (Rendering|Material|SetOverlayMaterial (Variables|Default|GetPlane) 0 :!class /Script/Engine.MeshComponent))))

(event Collision|EventActorBeginOverlap
  (params (OtherActor :type Actor%20Object%20Reference)))

(event EventTick
  (params (DeltaSeconds :type Float%20%28single-precision%29)))

(event EventInterract
  ;[1 1 1] Ramasser le masque
  (Audio|PlaySound2D "/Game/Assets/EventScripts/Event_Sounds_Ambience/KeyPickUp.KeyPickUp" 1.0 1.0 0.0 0 0)
  (bind _asbp_first_person_character (Utilities|Casting|CastToBP_FirstPersonCharacter (Game|GetPlayerCharacter 0)))
  (Variables|/Game/FirstPerson/Blueprints/BP_FirstPersonCharacter.BP_FirstPersonCharacter_C|SetHasMask? _asbp_first_person_character true)
  (Actor|DestroyActor))

(fn ConstructionScript)