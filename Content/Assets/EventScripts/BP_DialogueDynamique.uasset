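; BP_DialogueDynamique is a one-shot trigger volume that launches a dialogue when the first-person player walks into it.
; On BeginPlay it converts its array of name enum values into strings.
; On the player's first overlap with the box, it creates a WB_DialogueDynamique widget with the sound, names and subtitle text, adds it to the viewport and destroys itself.
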(event OnComponentBeginOverlap(Box)
  (params (OverlappedComponent :type Primitive%20Component%20Object%20Reference) (OtherActor :type Actor%20Object%20Reference) (OtherComp :type Primitive%20Component%20Object%20Reference) (OtherBodyIndex :type Integer) (bFromSweep :type Boolean) (SweepResult :type Hit%20Result%20Structure%20%28by%20ref%29))
  (Utilities|Casting|CastToBP_FirstPersonCharacter OtherActor)
  (Utilities|FlowControl|DoOnce false
    (:Completed
      (bind _returnvalue (UserInterface|CreateWidget "/Game/UserInterface/WB_DialogueDynamique.WB_DialogueDynamique_C" 0 (Variables|Default|GetSound) (Variables|Default|GetNoms) (Variables|Default|GetTexte)))
      (UserInterface|Viewport|AddtoViewport _returnvalue 0)
      (Actor|DestroyActor))))

(event EventBeginPlay
  (Utilities|Casting|CastToBP_FirstPersonCharacter (Game|GetPlayerCharacter 0))
  (for _array_element (Variables|Default|GetNom)
    (Utilities|Array|Add (Variables|Default|GetNoms) (Utilities|String|EnumtoString _array_element))))

(event Collision|EventActorBeginOverlap
  (params (OtherActor :type Actor%20Object%20Reference)))

(event EventTick
  (params (DeltaSeconds :type Float%20%28single-precision%29)))

(fn ConstructionScript)