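; Demo bad-ending trigger that shows the spotted game-over screen about two minutes after the first-person character enters its box.
; Box overlap opens a Gate and starts TimeBeforeDeath, which re-calls itself after a one-second Delay, incrementing a counter and printing a debug string.
; Once the counter passes 120, it adds WB_GameOver_Spotted to the viewport.
; ClosedGate can halt the countdown, but nothing here calls it.
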(event OnComponentBeginOverlap(Box)
  (params (OverlappedComponent :type Primitive%20Component%20Object%20Reference) (OtherActor :type Actor%20Object%20Reference) (OtherComp :type Primitive%20Component%20Object%20Reference) (OtherBodyIndex :type Integer) (bFromSweep :type Boolean) (SweepResult :type Hit%20Result%20Structure%20%28by%20ref%29))
  (Utilities|Casting|CastToBP_FirstPersonCharacter OtherActor)
  (CallFunction|OpenGate)
  (CallFunction|TimeBeforeDeath))

(event Custom|TimeBeforeDeath
  (Utilities|FlowControl|Gate true
    (:Exit
      (if (> (Variables|Default|GetTimerBeforeDeath) 120)
        (bind _returnvalue (UserInterface|CreateWidget "/Game/UserInterface/Mask/WB_GameOver_Spotted.WB_GameOver_Spotted_C"))
        (UserInterface|Viewport|AddtoViewport _returnvalue 0)
        (else
          (Utilities|FlowControl|Delay 1.0)
          (Math|Integer|IncrementInt (Variables|Default|GetTimerBeforeDeath)
            (:%20%20
              (Development|PrintString "Hello")
              (CallFunction|TimeBeforeDeath))))))))

(event Custom|ClosedGate
  (Utilities|FlowControl|Gate true) ; enters at Close
)

(event Custom|OpenGate
  (Utilities|FlowControl|Gate true) ; enters at Open
)

(event EventBeginPlay
  (Variables|Default|SetTimerBeforeDeath 0))

(event Collision|EventActorBeginOverlap
  (params (OtherActor :type Actor%20Object%20Reference)))

(event EventTick
  (params (DeltaSeconds :type Float%20%28single-precision%29)))

(fn ConstructionScript)